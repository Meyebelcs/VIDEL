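; Showcase Blueprint for the East Command 9S552 vehicle, exposing its animation and appearance options to showcase controls.
; Slider events forward values to setters, defined outside this graph, for wheels, hatches, doors, window cleaner, antenna rotation and light emissivity.
; The checkbox event toggles the damaged look, and the button index becomes a float to select the skin.
; BeginPlay is disabled and the construction script only calls its parent.
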(event EventBeginPlay
  (|CallParentFunction) ; This node is disabled and will not be called.\nDrag off pins to build functionality.
)

(event EventSetSliderVariable7
  (params (NewValue :type Float%20%28double-precision%29))
  ;[1 1 1] Showcase sliders
  (CallFunction|SetAntennaRotation NewValue))

(event EventSetButtonsVariable0
  (params (NewIndex :type Integer))
  ;[1 1 1] Showcase buttons
  (CallFunction|SetSkinType (Math|Conversions|ToFloat(Integer) NewIndex)))

(event EventSetSliderVariable6
  (params (NewValue :type Float%20%28double-precision%29))
  ;[1 1 1] Showcase sliders
  (CallFunction|SetWindowCleanerAngle NewValue))

(event EventSetSliderVariable5
  (params (NewValue :type Float%20%28double-precision%29))
  ;[1 1 1] Showcase sliders
  (CallFunction|BackandSideDoorAngle NewValue))

(event EventSetSliderVariable0
  (params (NewValue :type Float%20%28double-precision%29))
  ;[1 1 1] Showcase sliders
  (CallFunction|SetWheelSpeed NewValue))

(event EventSetSliderVariable1
  (params (NewValue :type Float%20%28double-precision%29))
  ;[1 1 1] Showcase sliders
  (CallFunction|SetWheelAngle NewValue))

(event EventSetSliderVariable2
  (params (NewValue :type Float%20%28double-precision%29))
  ;[1 1 1] Showcase sliders
  (CallFunction|SetHatchesAngle NewValue))

(event EventSetSliderVariable3
  (params (NewValue :type Float%20%28double-precision%29))
  ;[1 1 1] Showcase sliders
  (CallFunction|SetDoorsAngle NewValue))

(event EventSetSliderVariable4
  (params (NewValue :type Float%20%28double-precision%29))
  ;[1 1 1] Showcase sliders
  (CallFunction|SetLightsEmissivity NewValue))

(event EventSetCheckboxVariable0
  (params (NewState :type Boolean))
  ;[1 1 1] Showcase checkbox
  (CallFunction|SetShowDamaged NewState))

(fn ConstructionScript
  (|CallParentFunction))