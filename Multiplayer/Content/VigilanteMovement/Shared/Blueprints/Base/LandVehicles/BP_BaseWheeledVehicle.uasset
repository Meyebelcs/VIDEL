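; Base Chaos wheeled vehicle Blueprint that handles driving input, telemetry and toggleable all-wheel drive, with empty aim and turret hooks for child Blueprints.
; Input axes and actions drive steering, throttle or brake, and handbrake on the movement component.
; Tick records speed, velocity, engine RPM and an acceleration value, then updates the camera.
; When available, the Gears action toggles AWD, switching engine and handbrake effect on the first half of the wheels.
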(event Custom|UpdateSteering
  (params (Value :type Float%20%28double-precision%29))
  ;[1 1 1] Inputs from user and wheeled vehicle movements
  (Class|ChaosVehicleMovementComponent|SetSteeringInput (Variables|Default|GetChaosVehicleMovement) Value)
  (bind _returnvalue (Class|ChaosVehicleMovementComponent|GetThrottleInput (Variables|Default|GetChaosVehicleMovement)))
  (Variables|Internal|SetThrottle _returnvalue))

(event Custom|UpdateThrottle
  (params (Value :type Float%20%28double-precision%29))
  (bind _chaosvehiclemovement (Variables|Default|GetChaosVehicleMovement))
  ;[1 1 1] Inputs from user and wheeled vehicle movements
  (if (> Value 0.0)
    (Class|ChaosVehicleMovementComponent|SetThrottleInput _chaosvehiclemovement Value)
    (Class|ChaosVehicleMovementComponent|SetBrakeInput _chaosvehiclemovement 0.0)
    (else
      (bind _result (Math|Float|NegateFloat Value)
        (:%20%20
          (Class|ChaosVehicleMovementComponent|SetBrakeInput _chaosvehiclemovement _result)
          (Class|ChaosVehicleMovementComponent|SetThrottleInput _chaosvehiclemovement 0.0)))))
  (bind _returnvalue (Class|ChaosVehicleMovementComponent|GetThrottleInput (Variables|Default|GetChaosVehicleMovement)))
  (Variables|Internal|SetThrottle _returnvalue))

(event Custom|HandbrakeReleased
  ;[1 1 1] Inputs from user and wheeled vehicle movements
  (Class|ChaosVehicleMovementComponent|SetHandbrakeInput (Variables|Default|GetChaosVehicleMovement) false)
  (bind _returnvalue (Class|ChaosVehicleMovementComponent|GetThrottleInput (Variables|Default|GetChaosVehicleMovement)))
  (Variables|Internal|SetThrottle _returnvalue))

(event Custom|HandbrakePressed
  ;[1 1 1] Inputs from user and wheeled vehicle movements
  (Class|ChaosVehicleMovementComponent|SetHandbrakeInput (Variables|Default|GetChaosVehicleMovement) true)
  (bind _returnvalue (Class|ChaosVehicleMovementComponent|GetThrottleInput (Variables|Default|GetChaosVehicleMovement)))
  (Variables|Internal|SetThrottle _returnvalue))

(event Custom|ToggleAWD
  ;[1 1 1] Toggle All Wheel Drive
  (if (Variables|Basic|GethasAWD?)
    (if (Variables|Internal|GetIsAWD?)
      (Variables|Internal|SetIsAWD? false)
      (else
        (Variables|Internal|SetIsAWD? true)))
    (CallFunction|TypeOfWheelDrive)))

(event Custom|UpdateAim
  ;[1 1 1] Used by Child Actor BP to update specific Gun Rotation
)

(event EventBeginPlay
  ;[1 1 1] Sets WheelDriveType
  (|CallParentFunction)
  (CallFunction|TypeOfWheelDrive))

(event EventTick
  (params (DeltaSeconds :type Float%20%28single-precision%29))
  (bind _skeletalmesh (Variables|Default|GetSkeletalMesh))
  (bind _returnvalue (Transformation|GetComponentVelocity _skeletalmesh))
  (bind (_x _y) (Math|Vector|BreakVector _returnvalue))
  ;[1 1 1] Calculates Speed and Velocity (X and Y) every frame
  (|CallParentFunction DeltaSeconds)
  (Variables|Internal|SetSpeed (Math|Vector|VectorLength _returnvalue))
  (Variables|Internal|SetX_Velocity _x)
  (Variables|Internal|SetY_Velocity _y)
  ;[1 1 1] Calculates Acceleration based on (V2-V1)/At
  (Variables|Internal|SetAcceleration (/ DeltaSeconds (- (Variables|Internal|GetSpeed) (Variables|Internal|GetSpeed_LastFrame))))
  (Variables|Internal|SetSpeed_LastFrame (Variables|Internal|GetSpeed))
  (CallFunction|UpdateCamera)
  ;[1 1 1] RPM
  (Variables|Internal|SetRPM (Class|ChaosWheeledVehicleMovementComponent|GetEngineRotationSpeed (Variables|Default|GetChaosVehicleMovement))))

(event Input|ActionEvents|InputActionHandbrake
  (params (Key :type Key%20Structure))
  ;[1 1 1] Mapps Project Inputs to coresponding Events
  (:Pressed
    (CallFunction|Handbrakepressed))
  (:Released
    (CallFunction|Handbrakepressed)))

(event Input|ActionEvents|InputActionGears
  (params (Key :type Key%20Structure))
  ;[1 1 1] Mapps Project Inputs to coresponding Events
  (:Pressed
    (CallFunction|ToggleAWD)))

(event Input|AxisEvents|InputAxisMoveForward
  (params (AxisValue :type Float%20%28single-precision%29))
  ;[1 1 1] Mapps Project Inputs to coresponding Events
  (CallFunction|UpdateThrottle AxisValue))

(event Input|AxisEvents|InputAxisMoveRight
  (params (AxisValue :type Float%20%28single-precision%29))
  ;[1 1 1] Mapps Project Inputs to coresponding Events
  (CallFunction|UpdateSteering AxisValue))

(event Input|AxisEvents|InputAxisLookUp
  (params (AxisValue :type Float%20%28single-precision%29))
  ;[1 1 1] Mapps Project Inputs to coresponding Events
  (CallFunction|UpdateAim))

(event Input|AxisEvents|InputAxisLookAround
  (params (AxisValue :type Float%20%28single-precision%29))
  ;[1 1 1] Mapps Project Inputs to coresponding Events
  (CallFunction|UpdateAim))

(fn ConstructionScript)

(fn TypeOfWheelDrive
  (LocalVariables|SetL_WheelsToAdjust (- (/ (Utilities|Array|Length (Variables|/Script/ChaosVehicles.ChaosWheeledVehicleMovementComponent|GetWheels (Variables|Default|GetChaosVehicleMovement))) 2) 1))
  (for _index (range 0 (LocalVariables|GetL_WheelsToAdjust))
    (Class|ChaosWheeledVehicleMovementComponent|SetAffectedbyHandbrake (Variables|Default|GetChaosVehicleMovement) _index (Variables|Internal|GetIsAWD?))
    (Class|ChaosWheeledVehicleMovementComponent|SetAffectedbyEngine (Variables|Default|GetChaosVehicleMovement) _index (Variables|Internal|GetIsAWD?))))

(fn SetTurretYaw
  (params (Yaw :type Float%20%28double-precision%29))
  ;[1 1 1] Used in Child Actor to Set Gun Rotation
)

(fn SetTurretPitch
  (params (Pitch :type Float%20%28double-precision%29))
  ;[1 1 1] Used in Child Actor to Set Gun Rotation
)