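; Drivable Stryker APC vehicle Blueprint that extends a parent vehicle with turret animation, gun effects and wheel dust.
; Aim updates pass offset turret yaw and gun pitch to the animation instance, which also receives hatch angles.
; Gun Niagara effects toggle only while the weapon system's active weapon is the Gun.
; Each tick, eight per-wheel Niagara dust effects scale with wheel spin speed, dropping to zero when airborne or nearly still.
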(event Custom|SetHatchesAngle
  (params (HatchAngle :type Float%20%28single-precision%29))
  ;[1 1 1] Sets hatches angle
  (CallFunction|SetHatches (.Anim%20Instance (Variables|Default|GetAnim%20Instance)) HatchAngle))

(event EventBeginPlay
  ;[1 1 1] Set Animation Instance
  (|CallParentFunction)
  (CallFunction|AddEffectsReferences)
  (bind _asabp_west_apc_stryker (Utilities|Casting|CastTo (Components|SkeletalMesh|GetAnimInstance (Variables|Default|GetSkeletalMesh))))
  (Variables|Default|SetAnim%20Instance 0 _asabp_west_apc_stryker))

(event EventTick
  (params (DeltaSeconds :type Float%20%28single-precision%29))
  ;[1 1 1] Updates Wheels Dust
  (|CallParentFunction DeltaSeconds)
  (CallFunction|UpdateWheelsDust))

(event EventUpdateAim
  (bind _aimrotation (CallFunction|GetAim))
  (bind (_roll _pitch _yaw) (Math|Rotator|BreakRotator _aimrotation))
  ;[1 1 1] Updates position of gun and turret
  (CallFunction|SetTurretPitch (+ (Variables|Aim|GetTurretOffsetPitch) _pitch))
  (CallFunction|SetTurretYaw (+ (Variables|Aim|GetTurretOffsetYaw) _yaw)))

(event EventStarGunVFX
  ;[1 1 1] Activate/Desactivate Gun NS
  (if (Utilities|Enum|Equal(Enum) (Default|GetActiveWeaponName (Variables|Default|GetWeaponSystem)) (Utilities|Text|MakeLiteralText "Gun"))
    (Components|Activation|SetActive (Variables|Default|GetNS_Gun) true true)))

(event EventStopGunVFX
  ;[1 1 1] Activate/Desactivate Gun NS
  (if (Utilities|Enum|Equal(Enum) (Default|GetActiveWeaponName (Variables|Default|GetWeaponSystem)) (Utilities|Text|MakeLiteralText "Gun"))
    (Components|Activation|SetActive (Variables|Default|GetNS_Gun) false true)))

(fn ConstructionScript)

(fn SetTurretPitch
  (params (Pitch :type Float%20%28double-precision%29))
  ;[1 1 1] SetsMachineGunTurretPitch
  (|CallParentFunction Pitch)
  (Variables|Default|SetGun%20Pitch (.Anim%20Instance (Variables|Default|GetAnim%20Instance)) Pitch))

(fn SetTurretYaw
  (params (Yaw :type Float%20%28double-precision%29))
  ;[1 1 1] SetsMachineGunTurretYaw
  (|CallParentFunction Yaw)
  (Variables|Default|SetTurret%20Yaw (.Anim%20Instance (Variables|Default|GetAnim%20Instance)) Yaw))

(fn UpdateWheelsDust
  ;[1 1 1] For each Wheel
  (for (_array_element _array_index) (Variables|Default|GetWheels (Variables|Default|GetChaosVehicleMovement))
    (LocalVariables|SetL_Index _array_index)
    ;[1 1 1] Sets Final Dust Effect
    (if (and (.bInContact (CallFunction|BreakWheelStatus (CallFunction|GetWheelState (Variables|Default|GetChaosVehicleMovement) (LocalVariables|GetL_Index)))) (> (Math|Float|Absolute(Float) (CallFunction|GetRotationAngularVelocity _array_element)) 1.0))
      (Niagara|SetNiagaraVariable(Float) (Utilities|Array|Get(acopy) (Variables|Default|GetNS_WheelsVFX_Ref) (LocalVariables|GetL_Index)) "WheelSpeed" (* (Math|Float|Absolute(Float) (CallFunction|GetRotationAngularVelocity _array_element)) (Variables|Default|GetDustMultiplicator)))
      (else
        (Niagara|SetNiagaraVariable(Float) (Utilities|Array|Get(acopy) (Variables|Default|GetNS_WheelsVFX_Ref) (LocalVariables|GetL_Index)) "WheelSpeed" 0.0)))))

(fn AddEffectsReferences
  ;[1 1 1] Adds Referrences to Effects to Array to be used with Wheels
  (Variables|Default|SetNS_WheelsVFX_Ref (Utilities|Array|MakeArray (Variables|Default|GetNS_WheelDust_L1) (Variables|Default|GetNS_WheelDust_L2) (Variables|Default|GetNS_WheelDust_L3) (Variables|Default|GetNS_WheelDust_L4) (Variables|Default|GetNS_WheelDust_R1) (Variables|Default|GetNS_WheelDust_R2) (Variables|Default|GetNS_WheelDust_R3) (Variables|Default|GetNS_WheelDust_R4))))