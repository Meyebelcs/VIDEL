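; Showcase variant of the Stryker APC vehicle Blueprint that exposes its features to slider, checkbox and button controls.
; Events forward UI values to wheel spin and steering in the AnimInstance, turret aim, hatches, lights, damage mode, skin and weapon fire.
; The wheel speed slider also drives the wheel dust Niagara effects, scaled by a dust multiplier.
; UpdateWheelsDust is overridden empty, so the parent's dust update does not run.
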(event EventSetCheckboxVariable1
  (params (NewState :type Boolean))
  (bind _weaponsystem (Variables|Default|GetWeaponSystem))
  ;[1 1 1] Showcase checkboxes
  (if NewState
    (Default|StartFire _weaponsystem)
    (else
      (Default|StopFire _weaponsystem))))

(event EventSetSliderVariable0
  (params (NewValue :type Float%20%28double-precision%29))
  ;[1 1 1] Showcase sliders
  (bind _output_get (Variables|Default|SetWheel%20Speed (.Anim%20Instance (Variables|Default|GetAnim%20Instance)) NewValue))
  (for _array_element (Variables|Default|GetNS_WheelsVFX_Ref)
    (Niagara|SetNiagaraVariable(Float) _array_element "WheelSpeed" (* _output_get (Variables|Default|GetDustMultiplicator) 1.0))))

(event EventSetButtonsVariable0
  (params (NewIndex :type Integer))
  ;[1 1 1] Showcase buttons
  (CallFunction|SetSkinType NewIndex))

(event EventSetSliderVariable5
  (params (NewValue :type Float%20%28double-precision%29))
  ;[1 1 1] Showcase sliders
  (CallFunction|SetLightsIntensity NewValue))

(event EventSetSliderVariable4
  (params (NewValue :type Float%20%28double-precision%29))
  ;[1 1 1] Showcase sliders
  (CallFunction|SetHatchesAngle NewValue))

(event EventSetSliderVariable3
  (params (NewValue :type Float%20%28double-precision%29))
  ;[1 1 1] Showcase sliders
  (CallFunction|SetTurretPitch NewValue))

(event EventSetSliderVariable2
  (params (NewValue :type Float%20%28double-precision%29))
  ;[1 1 1] Showcase sliders
  (CallFunction|SetTurretYaw NewValue))

(event EventSetSliderVariable1
  (params (NewValue :type Float%20%28double-precision%29))
  ;[1 1 1] Showcase sliders
  (Variables|Default|SetFront%20Wheels%20Rotation (.Anim%20Instance (Variables|Default|GetAnim%20Instance)) NewValue))

(event EventSetCheckboxVariable0
  (params (NewState :type Boolean))
  ;[1 1 1] Showcase checkboxes
  (CallFunction|SetDamagedMode NewState))

(fn ConstructionScript
  (|CallParentFunction))

(fn UpdateWheelsDust)